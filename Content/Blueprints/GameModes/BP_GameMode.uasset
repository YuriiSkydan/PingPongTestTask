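; Game mode for a two-player match that assigns players to PlayerStart actors.
; ReadyToStartMatch allows the match to begin when exactly two players are counted.
; ChoosePlayerStart gathers all PlayerStarts and increments a running index on each call to pick the next one, with no bounds check or wrap.
; PostLogin only runs a one-second delay with nothing after it.
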(event `self.K2_PostLogin`
  (params (NewPlayer :type "PlayerController Object Reference"))
  (`KismetSystemLibrary.Delay` 1.0))

(fn `ChoosePlayerStart`
  (params (Player :type "Controller Object Reference"))
  (returns (ReturnValue :type "Actor Object Reference"))
  (bind _playerstartindex (`self.PlayerStartIndex`))
  (bind _outactors (`GameplayStatics.GetAllActorsOfClass` "/Script/Engine.PlayerStart"))
  (`/Engine/EditorBlueprintResources/StandardMacros.IncrementInt` _playerstartindex
    (:`  `
      (return (`|GetArrayItem` _outactors _playerstartindex)))))

(fn `ReadyToStartMatch`
  (returns (ReturnValue :type Boolean))
  (return (== (`self.NumPlayers`) 2)))

(fn `UserConstructionScript`)